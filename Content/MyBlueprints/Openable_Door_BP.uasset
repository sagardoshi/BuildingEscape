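; Openable door actor that swings open and closed in response to its OpenDoor component's events.
; BeginPlay saves the starting rotation so the swing angle stays relative to how the door is placed.
; OnOpen plays the DoorSwing timeline and OnClose reverses it, combining the animated yaw with that saved rotation.
; An event track on the timeline plays a quiet DoorClose sound at the door's location.
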(event OnOpen(OpenDoor)
  ;[1 1 1] Animate door opens/closes relative to original door angle
  (bind _open_angle (Timeline|Door%20Swing Play)
    (:Update
      (Transformation|SetActorRelativeRotation (Math|Rotator|CombineRotators (Math|Rotator|MakeRotator 0.0 0.0 _open_angle) (Variables|Default|GetInitial%20Rotation))))
    (:Sound%20Timing
      (Audio|PlaySoundatLocation "/Game/Audio/DoorClose.DoorClose" (Transformation|GetActorLocation) "0, 0, 0" 0.15))))

(event OnClose(OpenDoor)
  ;[1 1 1] Animate door opens/closes relative to original door angle
  (bind _open_angle (Timeline|Door%20Swing Reverse)
    (:Update
      (Transformation|SetActorRelativeRotation (Math|Rotator|CombineRotators (Math|Rotator|MakeRotator 0.0 0.0 _open_angle) (Variables|Default|GetInitial%20Rotation))))
    (:Sound%20Timing
      (Audio|PlaySoundatLocation "/Game/Audio/DoorClose.DoorClose" (Transformation|GetActorLocation) "0, 0, 0" 0.15))))

(event EventBeginPlay
  ;[1 1 1] Save Initial Rotations for Relative Door Angles
  (Variables|Default|SetInitial%20Rotation (Transformation|GetActorRotation)))

(fn ConstructionScript)