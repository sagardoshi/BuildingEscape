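; Triangular pyramid shape Blueprint that shows or hides a text dialogue when interacted with.
; The Interact event acts as a toggle, removing and clearing the stored 3DDialogue widget if it is valid.
; Otherwise it creates the widget for player 0, adds it to the viewport and passes MyText in as the dialogue text.
; Despite the widget's 3D name, it displays as a screen overlay.
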(event EventInteract
  (Utilities|IsValid (Variables|Default|Get3DDialogueWidget)
    (:Is%20Valid
      (Widget|RemovefromParent (Variables|Default|Get3DDialogueWidget))
      (Variables|Default|Set3DDialogueWidget 0))
    (:Is%20Not%20Valid
      (bind _returnvalue (UserInterface|CreateWidget "/Game/UI/3DDialogue.3DDialogue_C" (Game|GetPlayerController 0)))
      (bind _output_get (Variables|Default|Set3DDialogueWidget _returnvalue))
      (UserInterface|Viewport|AddtoViewport _output_get 0)
      (Variables|/Game/UI/3DDialogue.3DDialogue_C|SetDialogueText (Variables|Default|Get3DDialogueWidget) (Variables|Default|GetMyText)))))

(fn ConstructionScript)